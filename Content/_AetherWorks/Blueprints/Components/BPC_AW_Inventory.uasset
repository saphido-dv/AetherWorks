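; Inventory actor component that stores item stacks in a replicated array of slots.
; On BeginPlay the server fills an empty array with MaxSlots empty stacks, then adds and removes wood logs in slot 0, apparently as a test.
; Internal helpers set, clear, increase and decrease slots, clearing any stack that drops to zero or below.
; OnRep of the array fires the OnInventoryChanged dispatcher.
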(event EventBeginPlay
  ;[0.15 0.15 0.15 0.5] Initialization
  (|CallParentFunction)
  ;;[0 0 0 0.5] Check if inventory is not initialized (ONLY ON SERVER)
  (Networking|SwitchHasAuthority
    (:Authority
      (if (== (Utilities|Array|Length (Variables|Inventory|Data|GetInventorySlots)) 0)
        ;;[0 0 0 0.5] Initialize inventory slots. (ONLY ON SERVER)
        (Inventory|Internal|FInitializeInventory)
        (Inventory|Internal|FInternalSetSlot 0 (Utilities|Struct|MakeS_AW_ItemStack "/Game/_AetherWorks/Data/DataAssets/Items/PDA_AW_Item_WoodLog.PDA_AW_Item_WoodLog" 25))
        (Inventory|Internal|FInternalDecreaseQuantity 0 25)))))

(fn OnRepInventorySlots
  ;[0.15 0.15 0.15 0.5] Called whenever InventorySlots is replicated.
  (Default|CallEDonInventoryChanged))

(fn FInitializeInventory
  ;[0.15 0.15 0.15 0.5] Initializes the inventory by creating the configured number of empty slots.
  (Utilities|Array|Clear (Variables|Inventory|Data|GetInventorySlots))
  (for _index (range 0 (- (Variables|Inventory|Configuration|GetMaxSlots) 1))
    (Utilities|Array|Add (Variables|Inventory|Data|GetInventorySlots) (Utilities|Struct|MakeS_AW_ItemStack))))

(fn FInternalSetSlot
  (params (SlotIndex :type Integer) (ItemStack :type S%20AW%20Item%20Stack%20Structure))
  ;[0.15 0.15 0.15 0.5] Replaces the content of a slot.
  (Utilities|Array|SetArrayElem (Variables|Inventory|Data|GetInventorySlots) SlotIndex ItemStack)
  (return))

(fn FInternalClearSlot
  (params (SlotIndex :type Integer))
  ;[0.15 0.15 0.15 0.5] Clears an inventory slot.
  (Inventory|Internal|FInternalSetSlot SlotIndex (Utilities|Struct|MakeS_AW_ItemStack)))

(fn FInternalIncreaseQuantity
  (params (SlotIndex :type Integer) (Amount :type Integer))
  ;[0.15 0.15 0.15 0.5] Increases the quantity of an existing ItemStack.
  (bind _output_get (LocalVariables|SetLCurrentStack (Inventory|Queries|FGetSlot SlotIndex)))
  (bind _structout (Utilities|Struct|SetmembersinS_AW_ItemStack _output_get (+ (.Quantity (Utilities|Struct|BreakS_AW_ItemStack (LocalVariables|GetLCurrentStack))) Amount)))
  (Inventory|Internal|FInternalSetSlot SlotIndex _structout))

(fn FGetSlot
  (params (SlotIndex :type Integer))
  ;[0.15 0.15 0.15 0.5] Get Item Stack reference from inventory slot at the given index.
  (return (Utilities|Array|Get(acopy) (Variables|Inventory|Data|GetInventorySlots) SlotIndex)))

(fn FInternalDecreaseQuantity
  (params (SlotIndex :type Integer) (Amount :type Integer))
  ;[0.15 0.15 0.15 0.5] Removes quantity from an existing ItemStack.
  ; Automatically clears the slot when the quantity reaches zero.
  (LocalVariables|SetLCurrentStack (Inventory|Queries|FGetSlot SlotIndex))
  (if (<= (- (.Quantity (Utilities|Struct|BreakS_AW_ItemStack (LocalVariables|GetLCurrentStack))) Amount) 0)
    ;;[0 0 0 0.5] Clear slot if new quantity is less or equal to 0
    (Inventory|Internal|FInternalClearSlot SlotIndex)
    (else
      ;;[0 0 0 0.5] If it's not less or equal to 0, decrease quantity
      (bind _structout (Utilities|Struct|SetmembersinS_AW_ItemStack (LocalVariables|GetLCurrentStack) (- (.Quantity (Utilities|Struct|BreakS_AW_ItemStack (LocalVariables|GetLCurrentStack))) Amount)))
      (Inventory|Internal|FInternalSetSlot SlotIndex _structout))))