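; Base Blueprint for gatherable resource nodes that grant the player a resource when interacted with.
; Interact casts the instigator to BP_AW_Character, adds the node's ResourceID and ResourceAmount to its inventory component, then prints the resulting quantity.
; BeginFocus only prints a debug message, and gathering neither depletes nor destroys the node.
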(event EventBeginFocus
  (params (InstigatorCharacter :type Character%20Object%20Reference))
  ;[0.15 0.15 0.15 0.5] Focus Resource Node
  (Development|PrintString "Resource Focused"))

(event EventInteract
  (params (InstigatorCharacter :type Character%20Object%20Reference))
  ;[0.15 0.15 0.15 0.5] Resource Gathering
  ;;[0.15 0.15 0.15 0.5] Retrieve Player Inventory Component
  (bind _asbp_aw_character (Utilities|Casting|CastToBP_AW_Character InstigatorCharacter))
  ;;[0.15 0.15 0.15 0.5] Add Resource
  (Default|FAddResource (Variables|/Game/AetherWorks/Blueprints/Characters/BP_AW_Character.BP_AW_Character_C|GetAC_Inventory _asbp_aw_character) (Variables|Resource|GetResourceID) (Variables|Resource|GetResourceAmount))
  (bind _quantity (Default|FGetResourceQuantity (Variables|/Game/AetherWorks/Blueprints/Characters/BP_AW_Character.BP_AW_Character_C|GetAC_Inventory _asbp_aw_character) (Variables|Resource|GetResourceID)))
  (Development|PrintString (Utilities|String|ToString(Integer) _quantity)))

(fn ConstructionScript)