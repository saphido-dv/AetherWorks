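; BP_AW_Storage is a storage building that takes in all resources carried by the player who interacts with it.
; Interact casts the instigator to BP_AW_Character and passes its inventory component to F_DepositAllResources.
; That function adds each item to the storage's own inventory component, then clears the source list without checking whether the adds succeeded.
; Debug prints report the interaction and list the stored contents afterwards.
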(event EventBeginPlay
  (|CallParentFunction) ; This node is disabled and will not be called.\nDrag off pins to build functionality.
)

(event Collision|EventActorBeginOverlap
  (params (OtherActor :type Actor%20Object%20Reference))
  (|CallParentFunction OtherActor) ; This node is disabled and will not be called.\nDrag off pins to build functionality.
)

(event EventTick
  (params (DeltaSeconds :type Float%20%28single-precision%29))
  (|CallParentFunction DeltaSeconds) ; This node is disabled and will not be called.\nDrag off pins to build functionality.
)

(event EventInteract
  (params (InstigatorCharacter :type Character%20Object%20Reference))
  ;[0.15 0.15 0.15 0.5] ========== STORAGE INTERACTION ==========
  (Development|PrintString "STORAGE INTERACT")
  ;;[0.15 0.15 0.15 0.5] Retrieve Player Inventory
  (bind _asbp_aw_character (Utilities|Casting|CastToBP_AW_Character InstigatorCharacter))
  ;;[0.15 0.15 0.15 0.5] Deposit Resources
  (Inventory|FDepositAllResources (Variables|/Game/AetherWorks/Blueprints/Characters/BP_AW_Character.BP_AW_Character_C|GetAC_Inventory _asbp_aw_character))
  (Development|PrintString "Resources Deposited")
  (Inventory|FDebugInventory))

(fn ConstructionScript
  (|CallParentFunction))

(fn FDepositAllResources
  (params (SourceInventory :type BP%20AW%20Inventory%20Component%20Object%20Reference))
  (bind _items (Variables|/Game/AetherWorks/Blueprints/Components/BP_AW_InventoryComponent.BP_AW_InventoryComponent_C|GetItems SourceInventory))
  ;[0.15 0.15 0.15 0.5] Transfer Source Inventory Contents
  (for _array_element _items
    (Default|FAddResource (Variables|Default|GetAC_Inventory) (.ResourceID (Utilities|Struct|BreakS_AW_ItemStack _array_element)) (.Quantity (Utilities|Struct|BreakS_AW_ItemStack _array_element))))
  ;[0.15 0.15 0.15 0.5] Clear Source Inventory
  (Utilities|Array|Clear _items))

(fn FDebugInventory
  (for _array_element (Variables|/Game/AetherWorks/Blueprints/Components/BP_AW_InventoryComponent.BP_AW_InventoryComponent_C|GetItems (Variables|Default|GetAC_Inventory))
    (Development|PrintString (Utilities|String|Append (Utilities|String|ToString(Name) (.ResourceID (Utilities|Struct|BreakS_AW_ItemStack _array_element))) ": " (Utilities|String|ToString(Integer) (.Quantity (Utilities|Struct|BreakS_AW_ItemStack _array_element)))))))