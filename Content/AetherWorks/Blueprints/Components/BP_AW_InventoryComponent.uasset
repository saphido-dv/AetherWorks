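; Inventory component that stores resources as item stacks in a fixed number of slots, filled with empty entries by the authority on BeginPlay.
; Quantity checks and removal use the first matching stack, and removal empties the slot at zero or below.
; Adding merges into a matching stack with no size cap; otherwise it searches for an empty slot, but that write passes no index, so it does not target the found slot.
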(event EventBeginPlay
  ;[0.15 0.15 0.15 0.5] Initialize inventories on server side
  (Networking|SwitchHasAuthority
    (:Authority
      (Inventory|FInitializeInventory))))

(fn FInitializeInventory
  ;[0.15 0.15 0.15 0.5] ========== INVENTORY INITIALIZATION ==========
  ;                        Create Empty Inventory Slots
  (Utilities|Array|Clear (Variables|Inventory|GetItems))
  (for _index (range 0 (- (Variables|Inventory|GetInventorySize) 1))
    (Utilities|Array|Add (Variables|Inventory|GetItems) (Utilities|Struct|MakeS_AW_ItemStack "None" 0 true))))

(fn FGetResourceQuantity
  (params (ResourceID :type Name))
  ;[0.15 0.15 0.15 0.5] Returns the quantity of a resource stored in the inventory.
  (for _array_element (Variables|Inventory|GetItems)
    (if (== (.ResourceID (Utilities|Struct|BreakS_AW_ItemStack _array_element)) ResourceID)
      (return (.Quantity (Utilities|Struct|BreakS_AW_ItemStack _array_element))))))

(fn FHasResource
  (params (ResourceID :type Name) (RequiredQuantity :type Integer))
  ;[0.15 0.15 0.15 0.5] Checks whether the inventory contains the required amount of a resource.
  (bind _quantity (Inventory|FGetResourceQuantity ResourceID))
  (return (>= _quantity RequiredQuantity)))

(fn FRemoveResource
  (params (ResourceID :type Name) (Quantity :type Integer))
  ;[0.15 0.15 0.15 0.5] Removes resources from the inventory.
  ;;[0.15 0.15 0.15 0.5] Search Resource Stack
  (bind (_array_element _array_index) (Utilities|Array|ForEachLoopwithBreak (Variables|Inventory|GetItems) :!label _label)
    (:LoopBody
      (if (== (.ResourceID (Utilities|Struct|BreakS_AW_ItemStack _array_element)) ResourceID)
        (if (<= (- (.Quantity (Utilities|Struct|BreakS_AW_ItemStack _array_element)) Quantity) 0)
          (Utilities|Array|SetArrayElem (Variables|Inventory|GetItems) _array_index (Utilities|Struct|MakeS_AW_ItemStack "None" 0 true))
          (goto _label Break)
          (else
            (Utilities|Array|SetArrayElem (Variables|Inventory|GetItems) _array_index (Utilities|Struct|MakeS_AW_ItemStack (.ResourceID (Utilities|Struct|BreakS_AW_ItemStack _array_element)) (- (.Quantity (Utilities|Struct|BreakS_AW_ItemStack _array_element)) Quantity) false))
            (goto _label Break)))))))

(fn FAddResource
  (params (ResourceID :type Name) (Quantity :type Integer))
  ;[0.15 0.15 0.15 0.5] Adds resources to the inventory.
  (LocalVariables|SetbStackFound? false)
  (bind (_array_element _array_index) (Utilities|Array|ForEachLoopwithBreak (Variables|Inventory|GetItems) :!label _label)
    (:LoopBody
      ;;[0.15 0.15 0.15 0.5] Search Existing Resource Stack
      (if (and (== (.IsEmpty (Utilities|Struct|BreakS_AW_ItemStack _array_element)) false) (== (.ResourceID (Utilities|Struct|BreakS_AW_ItemStack _array_element)) ResourceID))
        (Utilities|Array|SetArrayElem (Variables|Inventory|GetItems) _array_index (Utilities|Struct|MakeS_AW_ItemStack (.ResourceID (Utilities|Struct|BreakS_AW_ItemStack _array_element)) (+ (.Quantity (Utilities|Struct|BreakS_AW_ItemStack _array_element)) Quantity) false))
        (LocalVariables|SetbStackFound? true)
        (goto _label Break)))
    (:Completed
      ;;[0.15 0.15 0.15 0.5] Find Empty Slot
      (if (not (LocalVariables|GetbStackFound?))
        (bind _array_element_2 (Utilities|Array|ForEachLoopwithBreak (Variables|Inventory|GetItems) :!label _label_2)
          (:LoopBody
            (if (.IsEmpty (Utilities|Struct|BreakS_AW_ItemStack _array_element_2))
              (Utilities|Array|SetArrayElem (Variables|Inventory|GetItems) 0 (Utilities|Struct|MakeS_AW_ItemStack ResourceID Quantity false))
              (goto _label_2 Break))))))))